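; BP_Door is an interactable door that the first-person player opens with the E key.
; A Box overlap with the player character's capsule shows a debug prompt and enables the key press, and leaving the box disables it.
; Pressing E while enabled plays the OpenDoor timeline, which drives the static mesh's relative yaw.
; The timeline only plays forward, with no closing logic.
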(event `self.Box.OnComponentBeginOverlap`
  (params (OverlappedComponent :type "PrimitiveComponent Object Reference") (OtherActor :type "Actor Object Reference") (OtherComp :type "PrimitiveComponent Object Reference") (OtherBodyIndex :type Integer) (bFromSweep :type Boolean) (SweepResult :type "HitResult Structure (by ref)"))
  (bind _asbp_first_person_character (cast `/Game/FirstPerson/Blueprints/BP_FirstPersonCharacter` OtherActor))
  (if (== (`Character.CapsuleComponent` _asbp_first_person_character) OtherComp)
    (`KismetSystemLibrary.PrintString` "Press E to Open")
    (set `self.CanPressE` true)))

(event `Key|E`
  (params (Key :type "Key Structure"))
  (bind _canpresse (`self.CanPressE`))
  (:`Pressed`
    (if _canpresse
      (`KismetSystemLibrary.PrintString` (`KismetStringLibrary.Conv_BoolToString` _canpresse))
      (bind (_direction _opendoor) (`Timeline|Open Door`)
        (:`Update`
          (`SceneComponent.K2_SetRelativeRotation` (`self.StaticMesh`) (`KismetMathLibrary.MakeRotator` 0.0 0.0 _opendoor) false false))))))

(event `self.Box.OnComponentEndOverlap`
  (params (OverlappedComponent :type "PrimitiveComponent Object Reference") (OtherActor :type "Actor Object Reference") (OtherComp :type "PrimitiveComponent Object Reference") (OtherBodyIndex :type Integer))
  (set `self.CanPressE` false))

(fn `UserConstructionScript`)