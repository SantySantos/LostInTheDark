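; BP_Chair is an anomaly prop chair that swivels and plays audio when StartAnomaly is triggered.
; On BeginPlay it adds the chair's starting yaw to DesireRotation to get an absolute target yaw.
; RotateObject steps the yaw up by a fixed amount, then waits a tick and calls itself until the target is reached, so the turn speed depends on frame rate.
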(event `self.ReceiveBeginPlay`
  (bind (_relativerotation_roll _relativerotation_pitch _relativerotation_yaw) (`KismetMathLibrary.BreakRotator` (`SceneComponent.RelativeRotation` (`self.Chair`))))
  ; Getting values in beingplay
  (bind _output_get (set `self.CurrentRotation` _relativerotation_yaw))
  (set `self.DesireRotation` (+ _output_get (`self.DesireRotation`))))

(event `/Game/Santy/Blueprints/Interfaces/BPI_Interactable.StartAnomaly`
  ; Activate Audio
  (`self.RotateObject`)
  (`AudioComponent.Play` (`self.Audio`) 0.0))

(event `RotateObject`
  (bind (_relativerotation_roll _relativerotation_pitch _relativerotation_yaw) (`KismetMathLibrary.BreakRotator` (`SceneComponent.RelativeRotation` (`self.Chair`))))
  ; Rotating the chair
  (if (< _relativerotation_yaw (`self.DesireRotation`))
    (`SceneComponent.K2_AddRelativeRotation` (`self.Chair`) (`KismetMathLibrary.MakeRotator` 0.0 0.0 2.0) false false)
    (`KismetSystemLibrary.DelayUntilNextTick`)
    (`self.RotateObject`)))

(fn `UserConstructionScript`)