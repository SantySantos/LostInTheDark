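; BP_Eye is an eye actor for an anomaly in which every eye turns to face the player.
; StartAnomaly gathers all BP_Eye actors and points each at the first-person camera using a look-at rotation with a fixed pitch offset, applied as relative rotation.
; It re-calls itself through a next-tick delay inside the loop to keep tracking continuously, instead of using Event Tick.
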(event `/Game/Santy/Blueprints/Interfaces/BPI_Interactable.StartAnomaly`
  (bind _outactors (`GameplayStatics.GetAllActorsOfClass` "BP_Eye_C"))
  (bind _output_get (set `self.Eyes` _outactors))
  (for _array_element _output_get
    (`self.K2_SetActorRelativeRotation` _array_element (`KismetMathLibrary.MakeRotator` (.roll (`KismetMathLibrary.FindLookAtRotation` (`SceneComponent.K2_GetComponentLocation` (`Actor.RootComponent` _array_element)) (`SceneComponent.K2_GetComponentLocation` (`/Game/FirstPerson/Blueprints/BP_FirstPersonCharacter.FirstPersonCamera` (cast `/Game/FirstPerson/Blueprints/BP_FirstPersonCharacter` (`GameplayStatics.GetPlayerCharacter` 0) :!pure true))))) (- (.pitch (`KismetMathLibrary.FindLookAtRotation` (`SceneComponent.K2_GetComponentLocation` (`Actor.RootComponent` _array_element)) (`SceneComponent.K2_GetComponentLocation` (`/Game/FirstPerson/Blueprints/BP_FirstPersonCharacter.FirstPersonCamera` (cast `/Game/FirstPerson/Blueprints/BP_FirstPersonCharacter` (`GameplayStatics.GetPlayerCharacter` 0) :!pure true))))) 10.0) (.yaw (`KismetMathLibrary.FindLookAtRotation` (`SceneComponent.K2_GetComponentLocation` (`Actor.RootComponent` _array_element)) (`SceneComponent.K2_GetComponentLocation` (`/Game/FirstPerson/Blueprints/BP_FirstPersonCharacter.FirstPersonCamera` (cast `/Game/FirstPerson/Blueprints/BP_FirstPersonCharacter` (`GameplayStatics.GetPlayerCharacter` 0) :!pure true)))))) false false)
    (`KismetSystemLibrary.DelayUntilNextTick`)
    (`/Game/Santy/Blueprints/Interfaces/BPI_Interactable.StartAnomaly`)))

(fn `UserConstructionScript`)